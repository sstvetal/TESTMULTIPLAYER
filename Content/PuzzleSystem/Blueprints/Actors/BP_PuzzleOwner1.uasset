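; BP_PuzzleOwner1 is a puzzle owner actor that toggles a point light.
; On BeginPlay it initializes its ACPuzzleOwner component with its PuzzleID.
; The LightsOn event flips an On flag and switches the light intensity between lit and dark, and LightsTurnon simply forwards to it.
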(event Custom|LightsOn
  (bind _pointlight (Variables|Default|GetPointLight))
  (if (not (Variables|Default|GetOn))
    (Variables|Default|SetOn true)
    (Rendering|Components|Light|SetIntensity _pointlight 5e+03)
    (else
      (Variables|Default|SetOn false)
      (Rendering|Components|Light|SetIntensity _pointlight 0.0))))

(event EventLightsTurnon
  (CallFunction|Lightson))

(event EventBeginPlay
  (Default|Initialize (Variables|Default|GetAC_PuzzleOwner) (Variables|Default|GetPuzzleID)))

(fn ConstructionScript)