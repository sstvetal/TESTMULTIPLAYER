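; BP_PuzzleItem is a puzzle actor driven by an ACPuzzleItem component, initialized from PuzzleItemInfo in the construction script.
; Box overlaps register it as the player character's InteractedActor, or trigger it through other objects when PuzzleItemInfo allows.
; Interaction adds it to the puzzle, while an overlap count and flag help decide when leaving toggles its active state.
; The component's state-change event swaps the cube's material to show active or inactive.
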(event OnComponentBeginOverlap(Box)
  (params (OverlappedComponent :type Primitive%20Component%20Object%20Reference) (OtherActor :type Actor%20Object%20Reference) (OtherComp :type Primitive%20Component%20Object%20Reference) (OtherBodyIndex :type Integer) (bFromSweep :type Boolean) (SweepResult :type Hit%20Result%20Structure%20%28by%20ref%29))
  (Math|Integer|IncrementInt (Variables|Default|GetOverlapedComponents)
    (:%20%20
      (if (== (Game|GetPlayerCharacter 0) OtherActor)
        (bind _asbp_multiplayer_third_person_character (Utilities|Casting|CastToBP_MultiplayerThirdPersonCharacter OtherActor))
        (Variables|/Game/ThirdPerson/Blueprints/BP_MultiplayerThirdPersonCharacter.BP_MultiplayerThirdPersonCharacter_C|SetInteractedActor _asbp_multiplayer_third_person_character self)
        (elif (.InteractWithOtherObjects? (Utilities|Struct|BreakS_PuzzleItemInfo (Variables|Default|GetPuzzleItemInfo)))
          (Default|InteractedwithItem (Variables|Default|GetAC_PuzzleItem))
          (Variables|Default|SetOtherActor? true))))))

(event OnComponentEndOverlap(Box)
  (params (OverlappedComponent :type Primitive%20Component%20Object%20Reference) (OtherActor :type Actor%20Object%20Reference) (OtherComp :type Primitive%20Component%20Object%20Reference) (OtherBodyIndex :type Integer))
  (Math|Integer|DecrementInt (Variables|Default|GetOverlapedComponents)
    (:%20%20
      (if (<= (Variables|Default|GetOverlapedComponents) 0)
        (if (Variables|Default|GetOtherActor?)
          (Default|ChangeActiveState (Variables|Default|GetAC_PuzzleItem) :!label _label)
          (else
            (bind _asbp_multiplayer_third_person_character (Utilities|Casting|CastToBP_MultiplayerThirdPersonCharacter OtherActor :!label _label_2))
            (if (.InteractWithOtherObjects? (Utilities|Struct|BreakS_PuzzleItemInfo (Variables|Default|GetPuzzleItemInfo)))
              (goto _label)
              (else
                (Variables|/Game/ThirdPerson/Blueprints/BP_MultiplayerThirdPersonCharacter.BP_MultiplayerThirdPersonCharacter_C|SetInteractedActor _asbp_multiplayer_third_person_character 0)))))
        (else
          (goto _label_2))))))

(event Custom|StateChanged
  (params (Active? :type Boolean) (ItemActor :type Actor%20Object%20Reference))
  (bind _cube (Variables|Default|GetCube))
  (if Active?
    (Rendering|Material|SetMaterial _cube 0 "/Engine/BasicShapes/MyBasicShapeMaterial.MyBasicShapeMaterial")
    (else
      (Rendering|Material|SetMaterial _cube 0 "/Engine/BasicShapes/BasicShapeMaterial.BasicShapeMaterial"))))

(event EventBeginPlay
  (EventDispatchers|BindEventtoOnActiveStateChanged (Variables|Default|GetAC_PuzzleItem) (delegate Custom|StateChanged)))

(event EventInteractwithPuzzleItem
  (Default|AddItemtoPuzzle (Variables|Default|GetAC_PuzzleItem)))

(fn ConstructionScript
  (Default|Initialize (Variables|Default|GetAC_PuzzleItem) (Variables|Default|GetPuzzleItemInfo)))