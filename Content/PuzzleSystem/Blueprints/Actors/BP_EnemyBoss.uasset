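; BP_EnemyBoss is a boss enemy that wanders randomly and contributes an item to the puzzle system when destroyed.
; An AIMoveTo loop picks nearby reachable points, pausing briefly after each success; a failed move ends the loop.
; Incoming damage is printed and subtracted from CurrentHealth, destroying the actor at zero.
; Its ACPuzzleItem component is initialized with PuzzleItem at BeginPlay and calls AddItemToPuzzle on destruction.
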(event EventBeginPlay
  (Default|Initialize (Variables|Default|GetAC_PuzzleItem) (Variables|Default|GetPuzzle%20Item))
  (AI|AIMoveTo self (.RandomLocation (AI|Navigation|GetRandomReachablePointinRadius (Transformation|GetActorLocation) 1e+03 0 0)) 0 5.0 false :!label _label
    (:OnSuccess
      (Utilities|FlowControl|Delay 1.0)
      (goto _label))))

(event Game|Damage|EventAnyDamage
  (params (Damage :type Float%20%28single-precision%29) (DamageType :type Damage%20Type%20Object%20Reference) (InstigatedBy :type Controller%20Object%20Reference) (DamageCauser :type Actor%20Object%20Reference))
  (Development|PrintString (Utilities|String|ToString(Float) Damage) true true "(R=1.000000,G=0.000000,B=0.092665,A=1.000000)")
  (if (<= (- (Variables|Default|GetCurrentHealth) Damage) 0.0)
    (Actor|DestroyActor)
    (else
      (Variables|Default|SetCurrentHealth (- (Variables|Default|GetCurrentHealth) Damage)))))

(event EventDestroyed
  (Default|AddItemtoPuzzle (Variables|Default|GetAC_PuzzleItem)))

(fn ConstructionScript
  (|CallParentFunction))