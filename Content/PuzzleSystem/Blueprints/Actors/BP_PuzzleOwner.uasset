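; BP_PuzzleOwner is a puzzle-linked door actor that swings open and closed.
; On BeginPlay it initializes its ACPuzzleOwner component with a PuzzleID.
; OpenDoor forwards to DoorOpen, which toggles the Opened flag and plays the OpenCloseDoor timeline forward from start or in reverse from end.
; The timeline's track interpolates the door's relative yaw between 90 and 0 degrees.
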(event Custom|DoorOpen
  (if (not (Variables|Default|GetOpened?))
    (Variables|Default|SetOpened? true)
    (bind _openingdoor (Timeline|OpenCloseDoor PlayFromStart)
      (:Update
        (Transformation|SetRelativeRotation (Variables|Default|GetDoor) (Math|Rotator|MakeRotator 0.0 0.0 (Math|Float|Lerp 9e+01 0.0 _openingdoor)) false false)))
    (else
      (Variables|Default|SetOpened? false)
      (Timeline|OpenCloseDoor ReverseFromEnd))))

(event EventBeginPlay
  (Default|Initialize (Variables|Default|GetAC_PuzzleOwner) (Variables|Default|GetPuzzleID)))

(event EventOpenDoor
  (CallFunction|DoorOpen))

(fn ConstructionScript)