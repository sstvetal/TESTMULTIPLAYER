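; Actor component that makes its owner an interactable puzzle item, tracking its active state and reporting to BP_PuzzleManager.
; Interaction either toggles the item, registering it with the manager on activation, or, for ResetOtherItems items, toggles randomly picked items from the puzzle owner's interacted list.
; Timed items start a one-second looping countdown on activation.
; OnActiveStateChanged broadcasts deactivations, including timer expiry, which leaves the stored Active flag unchanged.
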(event Custom|InteractedWithItem
  (CallFunction|AddItemtoPuzzle))

(event Custom|StopPuzzleTimer
  (Utilities|Time|ClearandInvalidateTimerbyHandle (Variables|Default|GetPuzzleTimer))
  (Variables|Default|SetBaseTimeDuration 0.0)
  (Variables|Default|SetTimerIsActive? false)
  (Default|CallOnActiveStateChanged false (Components|GetOwner)))

(event Custom|StartPuzzleTImer
  (if (not (Variables|Default|GetTimerIsActive?))
    (Variables|Default|SetTimerIsActive? true)
    (bind _returnvalue (Utilities|Time|SetTimerbyEvent (delegate Custom|TimerBody) 1.0 true))
    (Variables|Default|SetPuzzleTimer _returnvalue)
    (else
      (CallFunction|StopPuzzleTimer))))

(event Custom|TimerBody
  (if (> (- (Variables|Default|GetTimeDuration) 1.0) 0.0)
    (Variables|Default|SetTimeDuration (- (Variables|Default|GetTimeDuration) 1.0))
    (else
      (CallFunction|StopPuzzleTimer))))

(event EventBeginPlay)

(event EventTick
  (params (DeltaSeconds :type Float%20%28single-precision%29)))

(fn Initialize
  (params (PuzzleItem :type S%20Puzzle%20Item%20Info%20Structure))
  (Variables|Default|SetPuzzleItem PuzzleItem)
  (bind _returnvalue (Actor|GetActorOfClass "/Game/PuzzleSystem/Blueprints/Actors/BP_PuzzleManager.BP_PuzzleManager_C"))
  (Variables|Default|SetPuzzleManagerRef _returnvalue)
  (Variables|Default|SetHas%20Timer? (.HasTimer (Utilities|Struct|BreakS_PuzzleItemInfo (Variables|Default|GetPuzzleItem))))
  (Variables|Default|SetBaseTimeDuration (.TimerDur (Utilities|Struct|BreakS_PuzzleItemInfo (Variables|Default|GetPuzzleItem))))
  (Variables|Default|SetReset%20Other%20Items? (.ResetOtherItems? (Utilities|Struct|BreakS_PuzzleItemInfo (Variables|Default|GetPuzzleItem)))))

(fn AddItemtoPuzzle
  (if (not (Variables|Default|GetReset%20Other%20Items?))
    (bind _canadd_ (CallFunction|ChangeActiveState))
    (if _canadd_
      (bind _puzzlemanagerref (Variables|Default|GetPuzzleManagerRef)
        (:then
          (Default|AddItemtoPazzle _puzzlemanagerref (Variables|Default|GetPuzzleItem) (Components|GetOwner)))
        (:else)))
    (else
      (bind _puzzlemanagerref_2 (Variables|Default|GetPuzzleManagerRef)
        (:then
          (bind (_founded_ _ownercomponent) (Default|GetPuzzleOwner _puzzlemanagerref_2 (.PuzzleID (Utilities|Struct|BreakS_PuzzleItemInfo (Variables|Default|GetPuzzleItem)))))
          (if _founded_
            (if (not (Utilities|Array|IsEmpty (Variables|/Game/PuzzleSystem/Blueprints/Components/AC_PuzzleOwner.AC_PuzzleOwner_C|GetPuzzleItemsInteracted _ownercomponent)))
              (LocalVariables|SetLocalPuzzleItems (Variables|/Game/PuzzleSystem/Blueprints/Components/AC_PuzzleOwner.AC_PuzzleOwner_C|GetPuzzleItemsInteracted _ownercomponent))
              (if (> (Utilities|Array|Length (Variables|/Game/PuzzleSystem/Blueprints/Components/AC_PuzzleOwner.AC_PuzzleOwner_C|GetPuzzleItemsInteracted _ownercomponent)) 0)
                (for _index (range 0 (Math|Random|RandomIntegerinRange 0 (- (Utilities|Array|Length (Variables|/Game/PuzzleSystem/Blueprints/Components/AC_PuzzleOwner.AC_PuzzleOwner_C|GetPuzzleItemsInteracted _ownercomponent)) 1)))
                  (Default|CallOnActiveStateChanged false (Utilities|Array|Get(acopy) (LocalVariables|GetLocalPuzzleItems) (Math|Random|RandomIntegerinRange 0 (- (Utilities|Array|Length (Variables|/Game/PuzzleSystem/Blueprints/Components/AC_PuzzleOwner.AC_PuzzleOwner_C|GetPuzzleItemsInteracted _ownercomponent)) 1))))
                  (CallFunction|ChangeActiveState (Actor|GetComponentbyClass (Utilities|Array|Get(acopy) (LocalVariables|GetLocalPuzzleItems) (Math|Random|RandomIntegerinRange 0 (- (Utilities|Array|Length (Variables|/Game/PuzzleSystem/Blueprints/Components/AC_PuzzleOwner.AC_PuzzleOwner_C|GetPuzzleItemsInteracted _ownercomponent)) 1))) "AC_PuzzleItem_C")))
                (else
                  (Default|CallOnActiveStateChanged false (Utilities|Array|Get(acopy) (Variables|/Game/PuzzleSystem/Blueprints/Components/AC_PuzzleOwner.AC_PuzzleOwner_C|GetPuzzleItemsInteracted _ownercomponent))))))))
        (:else)))))

(fn ChangeActiveState
  (if (.Active? (Utilities|Struct|BreakS_PuzzleItemInfo (Variables|Default|GetPuzzleItem)))
    (if (.CanBeDeactivated (Utilities|Struct|BreakS_PuzzleItemInfo (Variables|Default|GetPuzzleItem)))
      (bind _structout (Utilities|Struct|SetmembersinS_PuzzleItemInfo (Variables|Default|GetPuzzleItem) false))
      (Variables|Default|SetPuzzleItem _structout)
      (Default|CallOnActiveStateChanged false (Components|GetOwner))
      (return false)
      (else
        (return false)))
    (else
      (bind _structout_2 (Utilities|Struct|SetmembersinS_PuzzleItemInfo (Variables|Default|GetPuzzleItem) true))
      (Variables|Default|SetPuzzleItem _structout_2)
      (if (Variables|Default|GetHas%20Timer?)
        (Variables|Default|SetTimeDuration (Variables|Default|GetBaseTimeDuration))
        (CallFunction|StartPuzzleTImer)
        (return true)
        (else
          (return true))))))