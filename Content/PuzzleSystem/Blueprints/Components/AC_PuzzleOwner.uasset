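; Actor component that owns one puzzle, tracking item objectives and triggering its owner's reaction: open door, load level, turn on lights or spawn boss.
; Initialization registers it with BP_PuzzleManager by PuzzleID and copies the matching DT_Puzzle row.
; Added items increment objective counts and bind active-state changes, which recheck completion or remove deactivated items, un-solving repeatable puzzles.
; Owner reactions go through message calls; ResetItems is an empty stub.
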(event EventBeginPlay)

(event EventTick
  (params (DeltaSeconds :type Float%20%28single-precision%29)))

(fn Initialize
  (params (PuzzleID :type E_PuzzleID%20Enum :default "NewEnumerator0"))
  (Variables|Default|SetPuzzle%20ID PuzzleID)
  (bind _returnvalue (Actor|GetActorOfClass "/Game/PuzzleSystem/Blueprints/Actors/BP_PuzzleManager.BP_PuzzleManager_C"))
  (Variables|Default|SetPuzzleManagerRef _returnvalue)
  (Default|AddPuzzleOwners (Variables|Default|GetPuzzleManagerRef) (Variables|Default|GetPuzzle%20ID) self)
  (CallFunction|GetPuzzleInfo)
  (EventDispatchers|BindEventtoOnPuzzleSolved (EventDispatchers|CreateEvent :!event PuzzleSolved)))

(fn GetPuzzleInfo
  (bind _outrownames (DataTable|GetDataTableRowNames "/Game/PuzzleSystem/Datatables/DT_Puzzle.DT_Puzzle"))
  (bind _array_element (Utilities|Array|ForEachLoopwithBreak _outrownames :!label _label)
    (:LoopBody
      (bind _returnvalue (Utilities|GetDataTableRow "/Game/PuzzleSystem/Datatables/DT_Puzzle.DT_Puzzle" _array_element)
        (:then
          (if (Utilities|Enum|Equal(Enum) (.PuzzleID (Utilities|Struct|BreakS_PuzzleInfo _returnvalue)) (Variables|Default|GetPuzzle%20ID))
            (LocalVariables|SetLocalPuzzleInfo _returnvalue)
            (LocalVariables|SetLocalFound true)
            (goto _label Break)))))
    (:Completed
      (if (LocalVariables|GetLocalFound)
        (Variables|Default|SetPuzzleInfo (LocalVariables|GetLocalPuzzleInfo))
        (else
          (Variables|Default|SetPuzzleInfo ""))))))

(fn PuzzleSolved
  (bind _returnvalue (Components|GetOwner))
  (switch Utilities|FlowControl|Switch|SwitchonE_PuzzleAction (.PuzzleAction (Utilities|Struct|BreakS_PuzzleInfo (Variables|Default|GetPuzzleInfo)))
    (:NewEnumerator1
      (Class|BPIPuzzle|OpenDoor(Message) _returnvalue))
    (:NewEnumerator2
      (Class|BPIPuzzle|LoadLevel(Message) _returnvalue (CallFunction|GetLevelName)))
    (:NewEnumerator3
      (Class|BPIPuzzle|LightsTurnon(Message) _returnvalue))
    (:NewEnumerator4
      (Class|BPIPuzzle|SpawnBoss(Message) _returnvalue))))

(fn AddItem
  (params (ItemActorToAdd :type Actor%20Object%20Reference) (ItemToAdd :type S%20Puzzle%20Item%20Info%20Structure))
  (bind _canadd_ (CallFunction|CheckforDuplicates ItemActorToAdd))
  (if _canadd_
    (bind _returnvalue (CallFunction|CheckforPuzzleItem ItemToAdd ItemActorToAdd))
    (if _returnvalue
      (bind _canadd__2 (CallFunction|CanAddItem ItemToAdd))
      (if _canadd__2
        (bind _returnvalue_2 (Utilities|Array|Add (Variables|Default|GetPuzzleItemsInteracted) ItemActorToAdd))
        (LocalVariables|SetLocalIndex _returnvalue_2)
        (for (_array_element _array_index) (.PuzzleObjective (Utilities|Struct|BreakS_PuzzleInfo (Variables|Default|GetPuzzleInfo)))
          (if (Utilities|Enum|Equal(Enum) (.PuzzleItemName (Utilities|Struct|BreakS_PuzzleObjective _array_element)) (.ItemName (Utilities|Struct|BreakS_PuzzleItemInfo ItemToAdd)))
            (Utilities|Array|SetArrayElem (.PuzzleObjective (Utilities|Struct|BreakS_PuzzleInfo (Variables|Default|GetPuzzleInfo))) _array_index (Utilities|Struct|MakeS_PuzzleObjective (.PuzzleItemName (Utilities|Struct|BreakS_PuzzleObjective _array_element)) (.EmountRequired (Utilities|Struct|BreakS_PuzzleObjective _array_element)) (+ (.CurrentAmount (Utilities|Struct|BreakS_PuzzleObjective _array_element)) 1)))))
        (EventDispatchers|BindEventtoOnActiveStateChanged (Actor|GetComponentbyClass (Utilities|Array|Get(acopy) (Variables|Default|GetPuzzleItemsInteracted) (LocalVariables|GetLocalIndex)) "/Game/PuzzleSystem/Blueprints/Components/AC_PuzzleItem.AC_PuzzleItem_C") (EventDispatchers|CreateEvent :!event OnChangingActiveState))
        (CallFunction|TrytoSlovePuzzle)
        (return true)
        (else
          (return false)))
      (else
        (return false)))
    (else
      (return false))))

(fn CheckforDuplicates
  (params (ItemToCheck :type Actor%20Object%20Reference))
  (bind _array_element (Utilities|Array|ForEachLoopwithBreak (Variables|Default|GetPuzzleItemsInteracted) :!label _label)
    (:LoopBody
      (if (== _array_element ItemToCheck)
        (LocalVariables|SetLocalFounded? true)
        (goto _label Break)))
    (:Completed
      (return (LocalVariables|GetLocalFounded?)))))

(fn CheckforPuzzleItem
  (params (S_PuzzleItemInfo :type S%20Puzzle%20Item%20Info%20Structure%20%28by%20ref%29) (ActorToCheck :type Actor%20Object%20Reference))
  (bind (_puzzleid _itemname _active_ _canbedeactivated _hastimer_ _timerduration _resetotheritems_) (Utilities|Struct|BreakS_PuzzleItemInfo S_PuzzleItemInfo))
  (for _array_element (.PuzzleObjective (Utilities|Struct|BreakS_PuzzleInfo (Variables|Default|GetPuzzleInfo)))
    (if (Utilities|Enum|Equal(Enum) (.PuzzleItemName (Utilities|Struct|BreakS_PuzzleObjective _array_element)) _itemname)
      (LocalVariables|SetLocalFound? true)
      (elif _resetotheritems_
        (CallFunction|ResetItems ActorToCheck)
        (return false))))
  (return (LocalVariables|GetLocalFound?)))

(fn ResetItems
  (params (ActorToCheck :type Actor%20Object%20Reference)))

(fn CanAddItem
  (params (ItemToCheck :type S%20Puzzle%20Item%20Info%20Structure))
  (bind (_canrepeat_ _solved_) (CallFunction|CheckforPuzzleState))
  (if _solved_
    (if _canrepeat_
      _
      (else
        (return false))))
  (bind _array_element (Utilities|Array|ForEachLoopwithBreak (.PuzzleObjective (Utilities|Struct|BreakS_PuzzleInfo (Variables|Default|GetPuzzleInfo))) :!label _label)
    (:LoopBody
      (if (and (<= (.EmountRequired (Utilities|Struct|BreakS_PuzzleObjective _array_element)) (.CurrentAmount (Utilities|Struct|BreakS_PuzzleObjective _array_element))) (Utilities|Enum|Equal(Enum) (.PuzzleItemName (Utilities|Struct|BreakS_PuzzleObjective _array_element)) (.ItemName (Utilities|Struct|BreakS_PuzzleItemInfo ItemToCheck))))
        (LocalVariables|SetLocalCompleted? false)
        (goto _label Break)))
    (:Completed
      (return (LocalVariables|GetLocalCompleted?)))))

(fn CheckforPuzzleState
  (bind _puzzleinfo (Variables|Default|GetPuzzleInfo))
  (bind (_puzzleid _puzzleobjective _puzzleaction _repetable_ _solved_) (Utilities|Struct|BreakS_PuzzleInfo _puzzleinfo))
  (return _repetable_ _solved_))

(fn OnChangingActiveState
  (params (Active? :type Boolean) (ItemActor :type Actor%20Object%20Reference))
  (if Active?
    (bind _solved_ (CallFunction|TrytoSlovePuzzle))
    (if _solved_
      (Default|CallOnPuzzleSolved))
    (else
      (bind _array_element (Utilities|Array|ForEachLoopwithBreak (Variables|Default|GetPuzzleItemsInteracted) :!label _label)
        (:LoopBody
          (if (== _array_element ItemActor)
            (bind (_array_element_2 _array_index) (Utilities|Array|ForEachLoopwithBreak (.PuzzleObjective (Utilities|Struct|BreakS_PuzzleInfo (Variables|Default|GetPuzzleInfo))) :!label _label_2)
              (:LoopBody
                (if (Utilities|Enum|Equal(Enum) (.PuzzleItemName (Utilities|Struct|BreakS_PuzzleObjective _array_element_2)) (.ItemName (Utilities|Struct|BreakS_PuzzleItemInfo (Variables|/Game/PuzzleSystem/Blueprints/Components/AC_PuzzleItem.AC_PuzzleItem_C|GetPuzzleItem (Actor|GetComponentbyClass _array_element "/Game/PuzzleSystem/Blueprints/Components/AC_PuzzleItem.AC_PuzzleItem_C")))))
                  (bind _result (Math|Integer|DecrementInt (.CurrentAmount (Utilities|Struct|BreakS_PuzzleObjective _array_element_2)))
                    (:%20%20
                      (bind _structout (Utilities|Struct|SetmembersinS_PuzzleObjective _array_element_2 _result))
                      (Utilities|Array|SetArrayElem (.PuzzleObjective (Utilities|Struct|BreakS_PuzzleInfo (Variables|Default|GetPuzzleInfo))) _array_index _structout)
                      (LocalVariables|SetLocalFound true)
                      (goto _label_2 Break)))))
              (:Completed
                (if (LocalVariables|GetLocalFound)
                  (bind _returnvalue (Utilities|Array|RemoveItem (Variables|Default|GetPuzzleItemsInteracted) _array_element))
                  (LocalVariables|SetLocalFound _returnvalue)
                  (goto _label Break)
                  (else
                    (goto _label Break)))))))
        (:Completed
          (if (LocalVariables|GetLocalFound)
            (if (and (.Repetable? (Utilities|Struct|BreakS_PuzzleInfo (Variables|Default|GetPuzzleInfo))) (.Solved? (Utilities|Struct|BreakS_PuzzleInfo (Variables|Default|GetPuzzleInfo))))
              (bind _structout_2 (Utilities|Struct|SetmembersinS_PuzzleInfo (Variables|Default|GetPuzzleInfo) false))
              (Variables|Default|SetPuzzleInfo _structout_2)
              (Default|CallOnPuzzleSolved))))))))

(fn TrytoSlovePuzzle
  (bind _array_element (Utilities|Array|ForEachLoopwithBreak (.PuzzleObjective (Utilities|Struct|BreakS_PuzzleInfo (Variables|Default|GetPuzzleInfo))) :!label _label)
    (:LoopBody
      (if (> (.EmountRequired (Utilities|Struct|BreakS_PuzzleObjective _array_element)) (.CurrentAmount (Utilities|Struct|BreakS_PuzzleObjective _array_element)))
        (LocalVariables|SetLocalNotCompleted true)
        (goto _label Break)))
    (:Completed
      (if (LocalVariables|GetLocalNotCompleted)
        (return false)
        (else
          (bind _structout (Utilities|Struct|SetmembersinS_PuzzleInfo (Variables|Default|GetPuzzleInfo) true))
          (Variables|Default|SetPuzzleInfo _structout)
          (return true))))))

(fn GetLevelName
  (return (.LevelName (Utilities|Struct|BreakS_PuzzleInfo (Variables|Default|GetPuzzleInfo)))))